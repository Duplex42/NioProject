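; BP_HPotion is a potion pickup for the jump-and-run course that the ALS player character collects by touching it.
; A Sphere overlap calls PickUp and passes the result to the character's PickupItem.
; PickUp returns PickupID if the actor is not already hidden, then hides it and disables collision and tick.
; The potion is never destroyed, as the DestroyActor call is unconnected.
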(event `self.Sphere.OnComponentBeginOverlap`
  (params (OverlappedComponent :type "PrimitiveComponent Object Reference") (OtherActor :type "Actor Object Reference") (OtherComp :type "PrimitiveComponent Object Reference") (OtherBodyIndex :type Integer) (bFromSweep :type Boolean) (SweepResult :type "HitResult Structure (by ref)"))
  (`/Engine/EditorBlueprintResources/StandardMacros.IsValid` OtherActor
    (:`Is Valid`
      (bind _asals_player_character_bp (cast `/Game/AdvancedLocomotionV2/Blueprints/ALS_Player_CharacterBP` OtherActor))
      (bind _item_id (`self.PickUp`))
      (`/Game/AdvancedLocomotionV2/Blueprints/ALS_Player_CharacterBP.PickupItem` _asals_player_character_bp _item_id))))

(fn `PickUp`
  (returns (Item_ID :type "/Game/AdrianStuff/Blueprints/Enums/E_Pickup Enum"))
  (if (not (`self.bHidden`))
    (`self.SetActorHiddenInGame` true)
    (`self.SetActorEnableCollision` false)
    (`self.SetActorTickEnabled` false)
    (return (`self.PickupID`))))

(fn `UserConstructionScript`)