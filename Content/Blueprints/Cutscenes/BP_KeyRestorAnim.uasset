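; Cutscene actor that plays a key restoration animation, animating a key's head and two ear pieces.
; PlayCutscene snaps the ALS player to an arrow, blocks movement, unhides the pieces and blends the view to this actor.
; A duration-scaled timeline moves and spins the head, slides the ears to their editor-placed positions and rotates the spring-arm camera.
; On finish, the view blends back to the player and movement is restored.
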(event `Play Cutscene`
  (bind (_rot_roll _rot_pitch) (`KismetMathLibrary.BreakRotator` (`self.GetRotVal` (`self.Ear Left`))))
  (bind (_rot_roll_2 _rot_pitch_2) (`KismetMathLibrary.BreakRotator` (`self.GetRotVal` (`self.Ear Left`))))
  (bind (_relativerotation_roll _relativerotation_pitch) (`KismetMathLibrary.BreakRotator` (`SceneComponent.RelativeRotation` (`self.Head`))))
  (bind (_relativelocation_x _relativelocation_y) (`KismetMathLibrary.BreakVector` (`SceneComponent.RelativeLocation` (`self.Head`))))
  (`TimelineComponent.SetPlayRate` (`self.Cutscene_TL`) (/ 4.0 (`self.Cutscene Duration`)))
  (bind _asals_player_character_bp (cast `/Game/AdvancedLocomotionV2/Blueprints/ALS_Player_CharacterBP` (`GameplayStatics.GetPlayerPawn` 0)))
  (`/Game/AdvancedLocomotionV2/Blueprints/ALS_Player_CharacterBP.Set Player Transform` _asals_player_character_bp (`SceneComponent.K2_GetComponentToWorld` (`self.Arrow`)))
  (set `/Game/AdvancedLocomotionV2/Blueprints/ALS_Player_CharacterBP.DoNotMove` true _asals_player_character_bp)
  (`SceneComponent.SetHiddenInGame` (`self.Head`) false false)
  (`SceneComponent.SetHiddenInGame` (`self.Ear Left`) false false)
  (`SceneComponent.SetHiddenInGame` (`self.Ear Right`) false false)
  (`PlayerController.SetViewTargetWithBlend` (`GameplayStatics.GetPlayerController` 0) self (`self.BlendInDuration`) "VTBlend_Linear" 0.0 false)
  (`KismetSystemLibrary.Delay` (`self.BlendInDuration`))
  (bind (_direction _straight_curve _hill_curve _camera_rot) (`Timeline|Cutscene_TL`)
    (:`Update`
      (`SceneComponent.K2_SetRelativeTransform` (`self.Head`) (`KismetMathLibrary.MakeTransform` (`KismetMathLibrary.MakeVector` _relativelocation_x _relativelocation_y (* (`self.HeadPosValue`) _hill_curve)) (`KismetMathLibrary.MakeRotator` _relativerotation_roll _relativerotation_pitch (* _straight_curve (`self.HeadRotValue`))) (`SceneComponent.RelativeScale3D` (`self.Head`))) false false)
      (bind _returnvalue (* _straight_curve (`self.EarLeftRotValue`)))
      (`SceneComponent.K2_SetRelativeRotation` (`self.Ear Left`) (`KismetMathLibrary.MakeRotator` _returnvalue _rot_pitch_2 _returnvalue) false false)
      (`SceneComponent.K2_SetRelativeLocation` (`self.Ear Left`) (`KismetMathLibrary.VLerp` (`self.EarLeftStartPos`) (`self.EarLeftEndPos`) _straight_curve) false false)
      (bind _returnvalue_2 (* _straight_curve (`self.EarRightRotValue`)))
      (`SceneComponent.K2_SetRelativeRotation` (`self.Ear Right`) (`KismetMathLibrary.MakeRotator` (`self.OneMinus` _returnvalue_2) _rot_pitch _returnvalue_2) false false)
      (`SceneComponent.K2_SetRelativeLocation` (`self.Ear Right`) (`KismetMathLibrary.VLerp` (`self.EarRightStartPos`) (`self.EarRightEndPos`) _straight_curve) false false)
      (`SceneComponent.K2_SetRelativeRotation` (`self.SpringArm`) (`KismetMathLibrary.MakeRotator` (.x _camera_rot) (.y _camera_rot) (.z _camera_rot)) false false))
    (:`Finished`
      (`PlayerController.SetViewTargetWithBlend` (`GameplayStatics.GetPlayerController` 0) _asals_player_character_bp (`self.BlendOutDuration`) "VTBlend_Linear" 0.0 false)
      (`KismetSystemLibrary.Delay` (`self.BlendOutDuration`))
      (set `/Game/AdvancedLocomotionV2/Blueprints/ALS_Player_CharacterBP.DoNotMove` false _asals_player_character_bp))))

(fn `UserConstructionScript`
  (`SceneComponent.K2_SetRelativeTransform` (`self.Arrow`) (`self.Player Pos`) false false)
  (set `self.EarLeftEndPos` (`SceneComponent.RelativeLocation` (`self.Ear Left`)))
  (set `self.EarRightEndPos` (`SceneComponent.RelativeLocation` (`self.Ear Right`)))
  (`SceneComponent.K2_SetRelativeLocation` (`self.Ear Left`) (`self.EarLeftStartPos`) false false)
  (`SceneComponent.K2_SetRelativeLocation` (`self.Ear Right`) (`self.EarRightStartPos`) false false))