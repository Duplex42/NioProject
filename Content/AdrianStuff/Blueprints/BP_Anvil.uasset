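; BP_Anvil is an interactable anvil that plays a key restoration cutscene when the saved key data allows it.
; On Interact, it loads a Key_Data save object from the KeyDataSlot save slot if none is cached yet.
; It then queries that object's key result and plays the RestoreKeyAnim cutscene only when the result is true.
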(event `/Game/AdrianStuff/Blueprints/Interfaces/I_Interact.Interact`
  (`KismetSystemLibrary.PrintString` "Interact")
  (`/Engine/EditorBlueprintResources/StandardMacros.IsValid` (`self.Key_Data`)
    (:`Is Valid`
      _)
    (:`Is Not Valid`
      (bind _returnvalue (`GameplayStatics.LoadGameFromSlot` "KeyDataSlot"))
      (bind _askey_data (cast `/Game/DataTable/Key_Data` _returnvalue))
      (set `self.Key_Data` _askey_data)))
  (bind _all_found (`/Game/DataTable/Key_Data.GetKeyResult` (`self.Key_Data`)))
  (if _all_found
    (`/Game/AdrianStuff/Blueprints/Cutscenes/BP_KeyRestorAnim.Play Cutscene` (`self.RestoreKeyAnim`))))

(fn `UserConstructionScript`)