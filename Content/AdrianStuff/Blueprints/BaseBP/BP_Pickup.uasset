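; BP_Pickup is a base pickup actor that hovers, rotates and hands its PickupID to the ALS player character.
; BeginHover drives bobbing and spin from a timeline, with speeds and length adjustable through ChangeHoverRotSpeed.
; Overlapping PickupArea calls Pickup, which hides and disables the actor, then passes the ID to PickupItem.
; AttractArea overlap only casts; the timeline lerp toward the player's camera is disconnected and never runs.
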(event `Begin Hover`
  (`TimelineComponent.SetPlayRate` (`self.Hover_TL`) (`self.HoverSpeed`))
  (bind (_direction _hover_z) (`Timeline|Hover_TL`)
    (:`Update`
      (`/Engine/EditorBlueprintResources/StandardMacros.IsValid` self
        (:`Is Valid`
          (`self.K2_SetActorLocationAndRotation` (+ (`self.K2_GetActorLocation`) (`KismetMathLibrary.MakeVector` 0.0 0.0 (* _hover_z (`self.HoverLenght`)))) (`KismetMathLibrary.ComposeRotators` (`KismetMathLibrary.MakeRotator` 0.0 0.0 (`self.RotationSpeed`)) (`self.K2_GetActorRotation`)) true))))))

(event `self.AttractArea.OnComponentBeginOverlap`
  (params (OverlappedComponent :type "PrimitiveComponent Object Reference") (OtherActor :type "Actor Object Reference") (OtherComp :type "PrimitiveComponent Object Reference") (OtherBodyIndex :type Integer) (bFromSweep :type Boolean) (SweepResult :type "HitResult Structure (by ref)"))
  (bind _asals_player_character_bp (cast `/Game/AdvancedLocomotionV2/Blueprints/ALS_Player_CharacterBP` OtherActor)))

(event `self.PickupArea.OnComponentBeginOverlap`
  (params (OverlappedComponent :type "PrimitiveComponent Object Reference") (OtherActor :type "Actor Object Reference") (OtherComp :type "PrimitiveComponent Object Reference") (OtherBodyIndex :type Integer) (bFromSweep :type Boolean) (SweepResult :type "HitResult Structure (by ref)"))
  (bind _asals_player_character_bp (cast `/Game/AdvancedLocomotionV2/Blueprints/ALS_Player_CharacterBP` OtherActor))
  (bind _item_id (`self.Pickup`))
  (`/Game/AdvancedLocomotionV2/Blueprints/ALS_Player_CharacterBP.PickupItem` _asals_player_character_bp _item_id))

(fn `ChangeHoverRotSpeed`
  (params (`Hover Speed` :type "Float (double-precision)") (`Hover Lenght` :type "Float (double-precision)") (`Rotation Speed` :type "Float (double-precision)"))
  (set `self.HoverSpeed` `Hover Speed`)
  (set `self.HoverLenght` `Hover Lenght`)
  (set `self.RotationSpeed` `Rotation Speed`))

(fn `Pickup`
  (returns (Item_ID :type "/Game/AdrianStuff/Blueprints/Enums/E_Pickup Enum"))
  (if (not (`self.bHidden`))
    (`self.SetActorHiddenInGame` true)
    (`self.SetActorEnableCollision` false)
    (`self.SetActorTickEnabled` false)
    (return (`self.PickupID`))))

(fn `UserConstructionScript`)