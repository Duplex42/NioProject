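; Test potion pickup that hands its PickupID to the ALS player character's PickupItem when the player overlaps PickupArea.
; Pickup hides the actor and disables its collision and tick instead of destroying it.
; Timeline-driven hover-spin and pull toward the player's camera are present but disconnected, so BeginHover does nothing and AttractArea only casts.
; Setter functions store the hover, rotation and attraction tuning values.
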(event `Begin Hover`)

(event `self.AttractArea.OnComponentBeginOverlap`
  (params (OverlappedComponent :type "PrimitiveComponent Object Reference") (OtherActor :type "Actor Object Reference") (OtherComp :type "PrimitiveComponent Object Reference") (OtherBodyIndex :type Integer) (bFromSweep :type Boolean) (SweepResult :type "HitResult Structure (by ref)"))
  (bind _asals_player_character_bp (cast `/Game/AdvancedLocomotionV2/Blueprints/ALS_Player_CharacterBP` OtherActor)))

(event `self.PickupArea.OnComponentBeginOverlap`
  (params (OverlappedComponent :type "PrimitiveComponent Object Reference") (OtherActor :type "Actor Object Reference") (OtherComp :type "PrimitiveComponent Object Reference") (OtherBodyIndex :type Integer) (bFromSweep :type Boolean) (SweepResult :type "HitResult Structure (by ref)"))
  (bind _asals_player_character_bp (cast `/Game/AdvancedLocomotionV2/Blueprints/ALS_Player_CharacterBP` OtherActor))
  (bind _item_id (`self.Pickup`))
  (`/Game/AdvancedLocomotionV2/Blueprints/ALS_Player_CharacterBP.PickupItem` _asals_player_character_bp _item_id))

(fn `ChangeHoverRotSpeed`
  (params (`Hover Speed` :type "Float (double-precision)") (`Hover Lenght` :type "Float (double-precision)") (`Rotation Speed` :type "Float (double-precision)"))
  (set `self.HoverSpeed` `Hover Speed`)
  (set `self.HoverLenght` `Hover Lenght`)
  (set `self.RotationSpeed` `Rotation Speed`))

(fn `Pickup`
  (returns (Item_ID :type "/Game/AdrianStuff/Blueprints/Enums/E_Pickup Enum"))
  (if (not (`self.bHidden`))
    (`self.SetActorHiddenInGame` true)
    (`self.SetActorEnableCollision` false)
    (`self.SetActorTickEnabled` false)
    (return (`self.PickupID`))))

(fn `SetValues`
  (params (HoverSpeed :type "Float (double-precision)") (RotationSpeed :type "Float (double-precision)") (HoverLenght :type "Float (double-precision)") (AttractSpeed :type "Float (double-precision)"))
  (set `self.HoverSpeed` HoverSpeed)
  (set `self.RotationSpeed` RotationSpeed)
  (set `self.HoverLenght` HoverLenght)
  (set `self.AttractSpeed` AttractSpeed))

(fn `UserConstructionScript`)