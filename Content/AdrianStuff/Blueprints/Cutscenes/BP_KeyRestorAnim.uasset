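; BP_KeyRestorAnim is a cutscene actor that plays a key restoration animation and then gives the player a weapon.
; PlayCutscene snaps the player to an Arrow transform, locks movement, unhides the three key pieces and blends the camera to itself.
; It then plays its ActorSequence, whose stop event waits briefly, blends the view back, unlocks movement and calls AddWeaponForPlayer.
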(event `Play Cutscene`
  (bind _sequenceplayer (`ActorSequenceComponent.SequencePlayer` (`self.ActorSequence`)))
  (bind _asals_player_character_bp (cast `/Game/AdvancedLocomotionV2/Blueprints/ALS_Player_CharacterBP` (`GameplayStatics.GetPlayerPawn` 0)))
  (`/Game/AdvancedLocomotionV2/Blueprints/ALS_Player_CharacterBP.Set Player Transform` _asals_player_character_bp (`SceneComponent.K2_GetComponentToWorld` (`self.Arrow`)))
  (set `/Game/AdvancedLocomotionV2/Blueprints/ALS_Player_CharacterBP.DoNotMove` true _asals_player_character_bp)
  (`SceneComponent.SetHiddenInGame` (`self.Head`) false false)
  (`SceneComponent.SetHiddenInGame` (`self.Ear Left`) false false)
  (`SceneComponent.SetHiddenInGame` (`self.Ear Right`) false false)
  (`PlayerController.SetViewTargetWithBlend` (`GameplayStatics.GetPlayerController` 0) self (`self.BlendInDuration`) "VTBlend_Linear" 0.0 false)
  (`KismetSystemLibrary.Delay` (`self.BlendInDuration`))
  (`MovieSceneSequencePlayer.Play` _sequenceplayer)
  (add `MovieSceneSequencePlayer.OnStop` _sequenceplayer (delegate `OnStop`)))

(event `OnStop`
  (`KismetSystemLibrary.Delay` 1.5)
  (`PlayerController.SetViewTargetWithBlend` (`GameplayStatics.GetPlayerController` 0) (stale `Play Cutscene` _asals_player_character_bp) (`self.BlendOutDuration`) "VTBlend_Linear" 0.0 false)
  (`KismetSystemLibrary.Delay` (`self.BlendOutDuration`))
  (set `/Game/AdvancedLocomotionV2/Blueprints/ALS_Player_CharacterBP.DoNotMove` false (stale `Play Cutscene` _asals_player_character_bp))
  (`/Game/AdvancedLocomotionV2/Blueprints/ALS_Player_CharacterBP.Add Weapon For Player` (stale `Play Cutscene` _asals_player_character_bp)))

(fn `UserConstructionScript`)