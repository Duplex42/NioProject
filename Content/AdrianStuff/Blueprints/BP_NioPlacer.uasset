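; BP_NioPlacer is a one-shot cutscene trigger that places the player before a level sequence plays.
; Its Trigger event, gated by DoOnce, teleports the ALS player character to the Arrow component's location and rotation, plays the Sequencer's sequence and locks movement and camera.
; An EndPlay event bound to the sequence player's OnStop releases both locks, returning control to the player.
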(event `/Game/AdrianStuff/Blueprints/Interfaces/I_Triggerable.Trigger`
  (bind (_returnvalue_location _returnvalue_rotation) (`KismetMathLibrary.BreakTransform` (`SceneComponent.K2_GetComponentToWorld` (`self.Arrow`))))
  (bind _sequenceplayer (`LevelSequenceActor.SequencePlayer` (`self.Sequencer`)))
  (`/Engine/EditorBlueprintResources/StandardMacros.DoOnce` false
    (:`Completed`
      (bind _asals_player_character_bp (cast `/Game/AdvancedLocomotionV2/Blueprints/ALS_Player_CharacterBP` (`GameplayStatics.GetPlayerCharacter` 0)))
      (`/Game/AdvancedLocomotionV2/Blueprints/ALS_Player_CharacterBP.TeleportPlayer` _asals_player_character_bp _returnvalue_location _returnvalue_rotation)
      (`MovieSceneSequencePlayer.Play` _sequenceplayer)
      (add `MovieSceneSequencePlayer.OnStop` _sequenceplayer (delegate `End Play`))
      (bind _asals_player_character_bp_2 (cast `/Game/AdvancedLocomotionV2/Blueprints/ALS_Player_CharacterBP` (`GameplayStatics.GetPlayerCharacter` 0)))
      (set `/Game/AdvancedLocomotionV2/Blueprints/ALS_Player_CharacterBP.DoNotMove` true _asals_player_character_bp_2)
      (set `/Game/AdvancedLocomotionV2/Blueprints/ALS_Player_CharacterBP.DoNotMoveCamera` true _asals_player_character_bp_2))))

(event `End Play`
  (bind _asals_player_character_bp (cast `/Game/AdvancedLocomotionV2/Blueprints/ALS_Player_CharacterBP` (`GameplayStatics.GetPlayerCharacter` 0)))
  (set `/Game/AdvancedLocomotionV2/Blueprints/ALS_Player_CharacterBP.DoNotMove` false _asals_player_character_bp)
  (set `/Game/AdvancedLocomotionV2/Blueprints/ALS_Player_CharacterBP.DoNotMoveCamera` false _asals_player_character_bp))

(fn `UserConstructionScript`)