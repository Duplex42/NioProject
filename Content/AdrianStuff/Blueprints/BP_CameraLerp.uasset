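; BP_CameraLerp is an actor that serves as a view target for a scripted camera transition.
; Its Trigger event locks the ALS player character's movement, camera and jumping and hides its UI.
; It then starts a long cubic view-target blend to itself and immediately calls TransitionToMain on the ALS game mode, without waiting for the blend to finish.
; Nothing here restores control or the previous view.
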(event `/Game/AdrianStuff/Blueprints/Interfaces/I_Triggerable.Trigger`
  (bind _asals_player_character_bp (cast `/Game/AdvancedLocomotionV2/Blueprints/ALS_Player_CharacterBP` (`GameplayStatics.GetPlayerCharacter` 0)))
  (set `/Game/AdvancedLocomotionV2/Blueprints/ALS_Player_CharacterBP.DoNotMove` true _asals_player_character_bp)
  (set `/Game/AdvancedLocomotionV2/Blueprints/ALS_Player_CharacterBP.DoNotMoveCamera` true _asals_player_character_bp)
  (set `/Game/AdvancedLocomotionV2/Blueprints/ALS_Player_CharacterBP.DoNotJump` true _asals_player_character_bp)
  (`/Game/AdvancedLocomotionV2/Blueprints/ALS_Player_CharacterBP.SetUIVisibility` _asals_player_character_bp false)
  (`PlayerController.SetViewTargetWithBlend` (`GameplayStatics.GetPlayerController` 0) self 10.0 "VTBlend_Cubic" 0.0 false)
  (bind _asals_game_mode_bp (cast `/Game/AdvancedLocomotionV2/Blueprints/ALS_GameModeBP` (`GameplayStatics.GetGameMode`)))
  (`/Game/AdvancedLocomotionV2/Blueprints/ALS_GameModeBP.TransitionToMain` _asals_game_mode_bp))

(fn `UserConstructionScript`)