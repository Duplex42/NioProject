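; BP_Shop is an interactable shop actor, though its Interact event currently only validates and casts the player pawn to the ALS character.
; Unconnected logic prints a message, loads Key_Data from a save slot and plays a key-restore cutscene when the key result is true.
; A separate unconnected SpawnPotion call would spawn BP_HPotion at the Spawn component and launch it with a radial impulse.
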(event `/Game/AdrianStuff/Blueprints/Interfaces/I_Interact.Interact`
  (bind _returnvalue (`GameplayStatics.GetPlayerPawn` 0))
  (`/Engine/EditorBlueprintResources/StandardMacros.IsValid` _returnvalue
    (:`Is Valid`
      (cast `/Game/AdvancedLocomotionV2/Blueprints/ALS_Player_CharacterBP` _returnvalue))))

(fn `SpawnPotion`
  (bind _spawn (`self.Spawn`))
  (bind _returnvalue (`SceneComponent.K2_GetComponentLocation` _spawn))
  (bind (_returnvalue_x _returnvalue_y _returnvalue_z) (`KismetMathLibrary.BreakVector` (* (* _returnvalue (`SceneComponent.GetForwardVector` _spawn)) 100)))
  (bind _returnvalue_2 (`|SpawnActorFromClass` "/Game/TestPhase/JumpAndRunCourse/PickUp/BluePrints/BP_HPotion.BP_HPotion_C" (`KismetMathLibrary.Conv_VectorToTransform` _returnvalue) "Undefined" "OverrideRootScale" null null))
  (`PrimitiveComponent.AddRadialImpulse` (`/Game/TestPhase/JumpAndRunCourse/PickUp/BluePrints/BP_HPotion.Sphere` _returnvalue_2) (`KismetMathLibrary.MakeVector` _returnvalue_x _returnvalue_y (+ _returnvalue_z 100.0)) 1000.0 1000.0 "RIF_Constant" true))

(fn `UserConstructionScript`)