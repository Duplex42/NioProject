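; BP_ActivateFire is a trigger actor that grants the ALS player character fire magic.
; Trigger enables fire magic and debug fire shooting on player 0 and shows the can-shoot display on each call.
; A DoOnce makes the FireBall component explode and be destroyed only the first time.
; EndOverlapTrigger hides the display, leaving the ability enabled.
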(event `/Game/AdrianStuff/Blueprints/Interfaces/I_Triggerable.Trigger`
  (bind _fireball (`self.FireBall`))
  (bind _asals_player_character_bp (cast `/Game/AdvancedLocomotionV2/Blueprints/ALS_Player_CharacterBP` (`GameplayStatics.GetPlayerCharacter` 0)))
  (set `/Game/AdvancedLocomotionV2/Blueprints/ALS_Player_CharacterBP.CanShootDebugFire` true _asals_player_character_bp)
  (`/Game/AdvancedLocomotionV2/Blueprints/ALS_Player_CharacterBP.EnableFireMagic` _asals_player_character_bp true)
  (`/Game/AdvancedLocomotionV2/Blueprints/ALS_Player_CharacterBP.DisplayCanFireShoot` _asals_player_character_bp true)
  (`/Engine/EditorBlueprintResources/StandardMacros.DoOnce` false
    (:`Completed`
      (`GameplayStatics.SpawnEmitterAttached` "/Game/Nio_Souls_of_Desert/ParticleEffects/FantasyFireBall/P_ExplosionN.P_ExplosionN" _fireball)
      (`ActorComponent.K2_DestroyComponent` _fireball))))

(event `/Game/AdrianStuff/Blueprints/Interfaces/I_Triggerable.EndOverlapTrigger`
  (bind _asals_player_character_bp (cast `/Game/AdvancedLocomotionV2/Blueprints/ALS_Player_CharacterBP` (`GameplayStatics.GetPlayerCharacter` 0)))
  (`/Game/AdvancedLocomotionV2/Blueprints/ALS_Player_CharacterBP.DisplayCanFireShoot` _asals_player_character_bp false))

(fn `UserConstructionScript`)